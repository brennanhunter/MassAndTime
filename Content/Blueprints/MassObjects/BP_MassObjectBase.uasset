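; BP_MassObjectBase is a base Blueprint for objects that shrink and grow in discrete size steps.
; Shrink and Grow events each play a timeline that multiplies the Object component's scale from the last stored CurrentSize.
; On finish, the new scale is stored and the Size index steps, with checks keeping it between 0 and 2.
; A DoneGrowing flag blocks new resize requests while a scale change is running.
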(event `/Game/Blueprints/Interfaces/BPI_Scaleable.Shrink`
  (if (`self.DoneGrowing`)
    (bind (_direction _shrink) (`Timeline|ShrinkTimeline` :!via `PlayFromStart`)
      (:`Update`
        (if (> (`self.Size`) 0)
          (set `self.DoneGrowing` false)
          (`SceneComponent.SetRelativeScale3D` (`self.Object`) (* _shrink (`self.CurrentSize`)))))
      (:`Finished`
        (if (> (`self.Size`) 0)
          (set `self.CurrentSize` (`SceneComponent.RelativeScale3D` (`self.Object`)))
          (set `self.DoneGrowing` true)
          (set `self.Size` (- (`self.Size`) 1)))))))

(event `/Game/Blueprints/Interfaces/BPI_Scaleable.Grow`
  (if (`self.DoneGrowing`)
    (bind (_direction _grow) (`Timeline|GrowTimeline` :!via `PlayFromStart`)
      (:`Update`
        (if (< (`self.Size`) 2)
          (set `self.DoneGrowing` false)
          (`SceneComponent.SetRelativeScale3D` (`self.Object`) (* _grow (`self.CurrentSize`)))))
      (:`Finished`
        (if (< (`self.Size`) 2)
          (set `self.CurrentSize` (`SceneComponent.RelativeScale3D` (`self.Object`)))
          (set `self.DoneGrowing` true)
          (set `self.Size` (+ (`self.Size`) 1)))))))

(fn `UserConstructionScript`)