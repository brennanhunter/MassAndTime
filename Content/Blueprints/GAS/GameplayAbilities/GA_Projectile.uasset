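; GA_Projectile is a Gameplay Ability that casts a projectile spell from the third-person character.
; Gated by the player 0 character's CanCastSpell flag, it plays AM_SpellAttack and waits for the Event.Montage.Fireball gameplay event.
; That event spawns the AbilityChosen class at the avatar's RightHand socket, using the actor's rotation.
; The flag resets only when the montage completes, and the ability never calls EndAbility.
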(event `self.K2_ActivateAbility`
  (bind _asbp_third_person_character (cast `/Game/ThirdPerson/Blueprints/BP_ThirdPersonCharacter` (`GameplayStatics.GetPlayerCharacter` 0)))
  (bind _output_get (set `self.As BP Third Person Character` _asbp_third_person_character))
  (if (`/Game/ThirdPerson/Blueprints/BP_ThirdPersonCharacter.CanCastSpell` _output_get)
    (set `/Game/ThirdPerson/Blueprints/BP_ThirdPersonCharacter.CanCastSpell` false (`self.As BP Third Person Character`))
    (`AbilityTask_PlayMontageAndWait.CreatePlayMontageAndWaitProxy` "None" "/Game/Characters/Leonard/Animations/AM_SpellAttack.AM_SpellAttack"
      (:`then`
        (`AbilityTask_WaitGameplayEvent.WaitGameplayEvent` (struct :`TagName` "Event.Montage.Fireball") null
          (:`EventReceived`
            (bind _asbp_third_person_character_2 (cast `/Game/ThirdPerson/Blueprints/BP_ThirdPersonCharacter` (`self.GetAvatarActorFromActorInfo`)))
            (`|SpawnActorFromClass` (`self.AbilityChosen`) (`KismetMathLibrary.MakeTransform` (`SceneComponent.GetSocketLocation` (`Character.Mesh` _asbp_third_person_character_2) "RightHand") (`Actor.K2_GetActorRotation` _asbp_third_person_character_2)) "Undefined" "MultiplyWithRoot" null null))))
      (:`OnCompleted`
        (set `/Game/ThirdPerson/Blueprints/BP_ThirdPersonCharacter.CanCastSpell` true (`self.As BP Third Person Character`))))))